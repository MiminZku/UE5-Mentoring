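; BP_Mark is an animated marker actor that spins and bobs up and down in place.
; On BeginPlay it records its starting Z, then each Tick adds yaw at a constant rate scaled by delta time.
; A GoUp flag moves it vertically at constant speed between that start height and MoveLength above it, clamping at each end before reversing.
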(event EventBeginPlay
  (Variables|Default|SetstartZpos (.z (Transformation|GetActorLocation))))

(event Collision|EventActorBeginOverlap
  (params (OtherActor :type Actor%20Object%20Reference)))

(event EventTick
  (params (DeltaSeconds :type Float%20%28single-precision%29))
  (bind _returnvalue (Transformation|GetActorRotation))
  (bind _returnvalue_2 (Transformation|GetActorLocation))
  (bind _returnvalue_3 (Transformation|GetActorLocation))
  (bind _returnvalue_4 (Transformation|GetActorLocation))
  (bind _returnvalue_5 (* DeltaSeconds 5e+01))
  (bind _startzpos (Variables|Default|GetstartZpos))
  (bind _movelength (Variables|Default|GetmoveLength))
  (bind _startzpos_2 (Variables|Default|GetstartZpos))
  (bind _returnvalue_6 (+ _startzpos _movelength))
  (Transformation|SetActorRotation (Math|Rotator|MakeRotator (.roll _returnvalue) (.pitch _returnvalue) (+ (.yaw _returnvalue) (* DeltaSeconds 1e+02))))
  (if (Variables|Default|GetgoUp)
    (Transformation|SetActorLocation (Math|Vector|MakeVector (.x _returnvalue_4) (.y _returnvalue_4) (+ (.z _returnvalue_4) _returnvalue_5)) false false)
    (if (>= (.z _returnvalue_3) _returnvalue_6)
      (Transformation|SetActorLocation (Math|Vector|MakeVector (.x _returnvalue_3) (.y _returnvalue_3) _returnvalue_6) false false)
      (Variables|Default|SetgoUp false))
    (else
      (Transformation|SetActorLocation (Math|Vector|MakeVector (.x _returnvalue_4) (.y _returnvalue_4) (- (.z _returnvalue_4) _returnvalue_5)) false false)
      (if (<= (.z _returnvalue_2) _startzpos_2)
        (Transformation|SetActorLocation (Math|Vector|MakeVector (.x _returnvalue_2) (.y _returnvalue_2) _startzpos_2) false false)
        (Variables|Default|SetgoUp true)))))

(fn ConstructionScript)