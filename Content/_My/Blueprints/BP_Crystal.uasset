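; BP_Crystal is an interactable crystal pickup that offers the player an interaction while inside its sphere trigger.
; On overlap it sets the third-person character's interact type, crystal type from CrystalNum and a reference to itself, then enables the interaction prompt on the controller's main widget.
; Leaving the sphere resets the interact type, clears the reference and disables the prompt.
; The interaction itself is handled outside this Blueprint.
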(event OnComponentBeginOverlap(Sphere)
  (params (OverlappedComponent :type Primitive%20Component%20Object%20Reference) (OtherActor :type Actor%20Object%20Reference) (OtherComp :type Primitive%20Component%20Object%20Reference) (OtherBodyIndex :type Integer) (bFromSweep :type Boolean) (SweepResult :type Hit%20Result%20Structure%20%28by%20ref%29))
  (bind _asbp_third_person_character (Utilities|Casting|CastToBP_ThirdPersonCharacter OtherActor))
  (Variables|/Game/ThirdPerson/Blueprints/BP_ThirdPersonCharacter.BP_ThirdPersonCharacter_C|SetInteractType _asbp_third_person_character 2)
  (Variables|/Game/ThirdPerson/Blueprints/BP_ThirdPersonCharacter.BP_ThirdPersonCharacter_C|SetCrystalType _asbp_third_person_character (Variables|Default|GetCrystalNum))
  (Variables|/Game/ThirdPerson/Blueprints/BP_ThirdPersonCharacter.BP_ThirdPersonCharacter_C|SetCrystal _asbp_third_person_character self)
  (bind _asbp_adventure_girl_controller (Utilities|Casting|CastToBP_AdventureGirlController (Pawn|GetController _asbp_third_person_character)))
  (if (Utilities|IsValid (Variables|/Game/AdventureGirl/Demo/Blueprints/BP_AdventureGirlController.BP_AdventureGirlController_C|GetWB_Main _asbp_adventure_girl_controller))
    (Default|EnableInteraction (Variables|/Game/AdventureGirl/Demo/Blueprints/BP_AdventureGirlController.BP_AdventureGirlController_C|GetWB_Main _asbp_adventure_girl_controller))))

(event OnComponentEndOverlap(Sphere)
  (params (OverlappedComponent :type Primitive%20Component%20Object%20Reference) (OtherActor :type Actor%20Object%20Reference) (OtherComp :type Primitive%20Component%20Object%20Reference) (OtherBodyIndex :type Integer))
  (bind _asbp_third_person_character (Utilities|Casting|CastToBP_ThirdPersonCharacter OtherActor))
  (Variables|/Game/ThirdPerson/Blueprints/BP_ThirdPersonCharacter.BP_ThirdPersonCharacter_C|SetInteractType _asbp_third_person_character 0)
  (Variables|/Game/ThirdPerson/Blueprints/BP_ThirdPersonCharacter.BP_ThirdPersonCharacter_C|SetCrystal _asbp_third_person_character 0)
  (bind _asbp_adventure_girl_controller (Utilities|Casting|CastToBP_AdventureGirlController (Pawn|GetController _asbp_third_person_character)))
  (if (Utilities|IsValid (Variables|/Game/AdventureGirl/Demo/Blueprints/BP_AdventureGirlController.BP_AdventureGirlController_C|GetWB_Main _asbp_adventure_girl_controller))
    (Default|DisableInteraction (Variables|/Game/AdventureGirl/Demo/Blueprints/BP_AdventureGirlController.BP_AdventureGirlController_C|GetWB_Main _asbp_adventure_girl_controller))))

(event EventBeginPlay)

(event Collision|EventActorBeginOverlap
  (params (OtherActor :type Actor%20Object%20Reference)))

(event EventTick
  (params (DeltaSeconds :type Float%20%28single-precision%29)))

(fn ConstructionScript)