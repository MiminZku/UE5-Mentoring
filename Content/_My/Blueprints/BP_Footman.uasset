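; BP_Footman is an enemy character that performs a melee attack on the player.
; AttackPlayer sphere-traces forward for pawns and, on hitting BP_ThirdPersonCharacter, plays the footman attack montage and applies Damage immediately, without waiting for an animation notify.
; If the player's health is then zero or below, it clears the "player" Blackboard key by setting it to no object.
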(event Custom|Attack%20Player
  (bind _returnvalue (Transformation|GetActorLocation))
  (bind (_outhit _returnvalue_2) (Collision|SphereTraceForObjects _returnvalue (+ _returnvalue (* (Math|Vector|GetForwardVector (Transformation|GetActorRotation)) 2.5e+02)) 0.0 (Utilities|Array|MakeArray "ObjectTypeQuery3") false 0 "None"))
  (if _returnvalue_2
    (bind _asbp_third_person_character (Utilities|Casting|CastToBP_ThirdPersonCharacter (.HitActor (Collision|BreakHitResult _outhit))))
    (Development|PrintText "Attack!")
    (Animation|PlayAnimMontage "/Game/SkeletonArmy/Animations/Footman/AM_FootmanAtk.AM_FootmanAtk" 1.5 "None")
    (Game|Damage|ApplyDamage (.HitActor (Collision|BreakHitResult _outhit)) (Math|Conversions|ToFloat(Integer) (Variables|Default|GetDamage)) 0 0)
    (if (<= (Variables|/Game/ThirdPerson/Blueprints/BP_ThirdPersonCharacter.BP_ThirdPersonCharacter_C|GetHealth _asbp_third_person_character) 0.0)
      (AI|Components|Blackboard|SetValueasObject (AI|GetBlackboard 0) (Utilities|Name|MakeLiteralName "player") 0))))

(event EventBeginPlay)

(event Collision|EventActorBeginOverlap
  (params (OtherActor :type Actor%20Object%20Reference)))

(event EventTick
  (params (DeltaSeconds :type Float%20%28single-precision%29)))

(fn ConstructionScript)