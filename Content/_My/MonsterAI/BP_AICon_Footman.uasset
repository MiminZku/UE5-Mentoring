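; AI controller for the Footman monster that runs BT_Footman and feeds its blackboard.
; On begin play it stores the pawn's PatrolPivot location as "startLoc".
; Perception updates pass each actor to CheckPlayer, which only handles BP_ThirdPersonCharacter.
; CheckPlayer toggles the "player" key without reading sensed state: it clears a valid value, otherwise sets the character if its Health is above zero.
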(event OnPerceptionUpdated(AIPerception)
  (params (UpdatedActors :type Array%20of%20Actor%20Object%20References))
  (for _array_element UpdatedActors
    (CallFunction|CheckPlayer _array_element)))

(event EventBeginPlay
  (AI|RunBehaviorTree "/Game/_My/MonsterAI/BT_Footman.BT_Footman")
  (bind _asbp_footman (Utilities|Casting|CastToBP_Footman (Pawn|GetControlledPawn)))
  (AI|Components|Blackboard|SetValueasVector (AI|GetBlackboard 0) (Utilities|Name|MakeLiteralName "startLoc") (Transformation|GetActorLocation (Variables|/Game/_My/Blueprints/BP_Footman.BP_Footman_C|GetpatrolPivot _asbp_footman))))

(event EventTick
  (params (DeltaSeconds :type Float%20%28single-precision%29)))

(fn ConstructionScript)

(fn CheckPlayer
  (params (DetectedActor :type Actor%20Object%20Reference))
  (bind _asbp_third_person_character (Utilities|Casting|CastToBP_ThirdPersonCharacter DetectedActor))
  (Utilities|IsValid (AI|Components|Blackboard|GetValueasObject (AI|GetBlackboard 0) (Utilities|Name|MakeLiteralName "player"))
    (:Is%20Valid
      (Development|PrintText "Something gone")
      (AI|Components|Blackboard|SetValueasObject (AI|GetBlackboard 0) (Utilities|Name|MakeLiteralName "player") 0))
    (:Is%20Not%20Valid
      (if (> (Variables|/Game/ThirdPerson/Blueprints/BP_ThirdPersonCharacter.BP_ThirdPersonCharacter_C|GetHealth _asbp_third_person_character) 0.0)
        (Development|PrintText "Something detected")
        (AI|Components|Blackboard|SetValueasObject (AI|GetBlackboard 0) (Utilities|Name|MakeLiteralName "player") _asbp_third_person_character)))))